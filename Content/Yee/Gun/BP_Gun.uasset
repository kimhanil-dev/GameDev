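; BP_Gun is a data-driven gun that fires BP_Bullet projectiles, limited by capacity and fire rate.
; On BeginPlay it loads the first DT_Gun row into GunInfo and adds a component for each listed fixed state.
; FireEvent spawns bullets at the Muzzle socket with random cone spread narrowed by precision.
; The state components update the gun every tick, react to each shot, and are passed to the bullets.
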(event Custom|FireEvent
  (params (NewParam :type Float%20%28double-precision%29))
  (bind _guninfo (Variables|Default|GetgunInfo))
  (if (Variables|Default|GetisFireAllowed)
    (if (> (Variables|Default|Getcapacity) 0)
      (CallFunction|Fire)
      (Variables|Default|Setcapacity (- (Variables|Default|Getcapacity) (.bulletcount _guninfo)))
      (Variables|Default|SetisFireAllowed false)
      (Utilities|FlowControl|Delay (/ 1.0 (.firespeed _guninfo)))
      (Variables|Default|SetisFireAllowed true))))

(event EventBeginPlay
  (bind _guninfo (Variables|Default|GetgunInfo))
  (CallFunction|Load)
  (Variables|Default|Setcapacity (.maxcapacity _guninfo))
  (for _array_element (.statefixed _guninfo)
    (bind _returnvalue (Game|AddComponentbyClass _array_element))
    (Utilities|Array|Add (Variables|Default|GetstateFixed) _returnvalue)))

(event Collision|EventActorBeginOverlap
  (params (OtherActor :type Actor%20Object%20Reference)))

(event EventTick
  (params (DeltaSeconds :type Float%20%28single-precision%29))
  (for _array_element (Variables|Default|GetstateFixed)
    (Default|UpdateGun _array_element self)))

(fn ConstructionScript)

(fn Fire
  (bind _model (Variables|Default|GetModel))
  (bind _guninfo (Variables|Default|GetgunInfo))
  (bind _returnvalue (Transformation|GetSocketTransform _model "Muzzle" "RTS_World"))
  (for _index (range 1 (.bulletcount (Variables|Default|GetgunInfo)))
    (bind _returnvalue_2 (Game|SpawnActorfromClass "/Game/Yee/Gun/BP_Bullet.BP_Bullet_C" (Math|Transform|MakeTransform (.location _returnvalue) (.rotation _returnvalue) "1.000000,1.000000,1.000000") "AdjustIfPossibleButAlwaysSpawn" 0 0))
    (Variables|/Script/Engine.MovementComponent|SetVelocity (Variables|/Game/Yee/Gun/BP_Bullet.BP_Bullet_C|GetProjectileMovement _returnvalue_2) (* (Math|Random|RandomUnitVectorinConeinDegrees (Math|Vector|GetForwardVector (Variables|/Script/Engine.Actor|GetRootComponent _returnvalue_2)) (* (.fireangle _guninfo) (- 1.0 (.precision _guninfo)))) (Variables|Default|GetInitialSpeed)))
    (Variables|Default|SetisFireAllowed true)
    (for _array_element (Variables|Default|GetstateFixed)
      (Default|Fire _array_element self _returnvalue_2)
      (Variables|/Game/Yee/Gun/BP_Bullet.BP_Bullet_C|SetstateFixed _returnvalue_2 (Variables|Default|GetstateFixed)))))

(fn Load
  (params (id :type Integer))
  (bind _outrownames (DataTable|GetDataTableRowNames "/Game/Yee/Gun/DT_Gun.DT_Gun"))
  (bind _returnvalue (Utilities|GetDataTableRow "/Game/Yee/Gun/DT_Gun.DT_Gun" (Utilities|Array|Get(acopy) _outrownames id))
    (:then
      (Variables|Default|SetgunInfo _returnvalue))))