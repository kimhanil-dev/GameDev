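; BP_Weapon is a gun that spawns BP_Bullet at its muzzle socket, limited by fire delay and ammo.
; A looping timer re-enables firing every FireDelayTime, independent of when the last shot happened.
; BPStatus tracks ammo, while a Niagara shell effect, rate-matched to the delay, switches on in Fire and off in StopFire.
; Reload refills ammo and drops a physics-simulated empty magazine mesh with a limited lifespan.
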(event Custom|Reload
  (bind _mesh (Variables|Default|GetMesh))
  (Default|ResetCurrenttoMax (Variables|Default|GetBP_Status) "Ammo")
  ;[1 1 1] Visual Effect
  (bind _returnvalue (Game|SpawnActorfromClass "/Script/Engine.StaticMeshActor" (Math|Transform|MakeTransform (Transformation|GetSocketLocation _mesh "b_gun_mag") (Transformation|GetSocketRotation _mesh "b_gun_mag")) "AlwaysSpawn" (Components|GetOwner) 0))
  (Actor|SetLifeSpan _returnvalue 1e+01)
  (Transformation|SetMobility _returnvalue "Movable")
  (Components|StaticMesh|SetStaticMesh (Variables|/Script/Engine.StaticMeshActor|GetStaticMeshComponent _returnvalue) "/Game/Resources/FPS_Weapon_Bundle/Weapons/Meshes/Ka47/SM_KA47_Mag_Empty.SM_KA47_Mag_Empty")
  (Physics|SetEnableGravity (Variables|/Script/Engine.StaticMeshActor|GetStaticMeshComponent _returnvalue) true)
  (Physics|SetSimulatePhysics (Variables|/Script/Engine.StaticMeshActor|GetStaticMeshComponent _returnvalue) true))

(event Custom|Stop%20Fire
  (Effects|Components|ParticleSystem|SetBoolParameter (Variables|Default|GetNiagara) "IsFiring" false))

(event Custom|UpdateFireDelay
  ;[1 1 1] Init Attack DelayTime Timer
  (Variables|Default|SetIsCanFire true))

(event EventBeginPlay
  ;[1 1 1] Init Attack DelayTime Timer
  (bind _returnvalue (Utilities|Time|SetTimerbyEvent (delegate Custom|UpdateFireDelay) (Variables|Default|GetFireDelayTime) true))
  (Variables|Default|SetFireDelayTimer _returnvalue)
  ;[1 1 1] Init Sheel Effect SpawnRate
  (Effects|Components|ParticleSystem|SetFloatParameter (Variables|Default|GetNiagara) "SpawnRate" (/ 1.0 (Variables|Default|GetFireDelayTime)))
  (Default|AddVariable (Variables|Default|GetBP_Status) "Ammo" 5e+01 0.0 false))

(fn ConstructionScript)

(fn Fire
  (bind _mesh (Variables|Default|GetMesh))
  (if (Variables|Default|GetIsCanFire)
    (bind _isunderdeadline (Default|UpdateCurrent (Variables|Default|GetBP_Status) "Ammo" -1.0))
    (if (not _isunderdeadline)
      (Variables|Default|SetIsCanFire false)
      (Game|SpawnActorfromClass "/Game/Kim/Bullet/Blueprint/BP_Bullet.BP_Bullet_C" (Math|Transform|MakeTransform (Transformation|GetSocketLocation _mesh "Muzzle") (Transformation|GetSocketRotation _mesh "Muzzle")) "Undefined" (Components|GetOwner) 0)
      (Effects|Components|ParticleSystem|SetBoolParameter (Variables|Default|GetNiagara) "IsFiring" true))))