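; BP_Enemy is an enemy actor that tracks HP, takes damage and reports its death.
; BeginPlay registers HP in the BPStatus component, whose change events push values to the Widget, while AnyDamage subtracts from current HP.
; When HP hits its deadline, a valid enemy controller receives OnDead and BP_TopDownGameMode removes the enemy by index.
; GetCondition and SetAction are stubs that return false.
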(event Custom|OnMaxHPChange
  (params (NewCurrent :type Float%20%28double-precision%29))
  (Class|BPIVariableBind|UpdateVariable(Message) (UserInterface|GetWidget (Variables|Default|GetWidget)) NewCurrent "NewEnumerator3"))

(event Custom|OnDeadLine
  (bind _as_enemy_controller (Variables|Default|GetAs%20Enemy%20Controller))
  (Utilities|IsValid _as_enemy_controller
    (:Is%20Valid
      (Default|OnDead _as_enemy_controller)
      (bind _asbp_top_down_game_mode (Utilities|Casting|CastToBP_TopDownGameMode (Game|GetGameMode)))
      (Default|RemoveEnemy _asbp_top_down_game_mode (Variables|Default|GetEnemyIndex)))))

(event Custom|OnCurrentHPChange
  (params (NewCurrent :type Float%20%28double-precision%29))
  (Class|BPIVariableBind|UpdateVariable(Message) (UserInterface|GetWidget (Variables|Default|GetWidget)) NewCurrent "NewEnumerator0"))

(event EventBeginPlay
  (bind _bp_status (Variables|Default|GetBP_Status))
  ;[1 1 1] HP status init
  (Default|AddVariable _bp_status "HP" 5.0 0.0 false)
  (Default|BindonCurrentChangeEvent _bp_status "HP" (delegate Custom|OnCurrentHPChange))
  (Default|BindonMaxChangeEvent _bp_status "HP" (delegate Custom|OnMaxHPChange))
  (Default|BindonDeadLineEvent _bp_status "HP" (delegate Custom|OnDeadLine))
  (Default|CallFakeChangeEvent _bp_status))

(event Game|Damage|EventAnyDamage
  (params (Damage :type Float%20%28single-precision%29) (DamageType :type Damage%20Type%20Object%20Reference) (InstigatedBy :type Controller%20Object%20Reference) (DamageCauser :type Actor%20Object%20Reference))
  (Default|UpdateCurrent (Variables|Default|GetBP_Status) "HP" (* Damage -1.0)))

(event EventTick
  (params (DeltaSeconds :type Float%20%28single-precision%29)))

(event Collision|EventActorBeginOverlap
  (params (OtherActor :type Actor%20Object%20Reference)))

(fn ConstructionScript)

(fn GetCondition
  (params (ConditionName :type Name :default "None"))
  (return false))

(fn SetAction
  (params (ActionName :type Name :default "None"))
  (return false false))