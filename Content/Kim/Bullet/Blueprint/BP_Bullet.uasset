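; BP_Bullet is a projectile actor that damages what it overlaps and expires after a set lifetime.
; A sphere overlap with any actor not tagged Player spawns an explosion emitter, applies damage attributed to the bullet's owner, and destroys the bullet.
; A blocking hit also destroys it, unless the other actor is another bullet or the top-down character, with no damage or effect.
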(event OnComponentHit(Sphere)
  (params (HitComponent :type Primitive%20Component%20Object%20Reference) (OtherActor :type Actor%20Object%20Reference) (OtherComp :type Primitive%20Component%20Object%20Reference) (NormalImpulse :type Vector :default "0, 0, 0") (Hit :type Hit%20Result%20Structure%20%28by%20ref%29))
  (bind _returnvalue (Utilities|GetClass (.hitactor Hit)))
  (if (and (!= _returnvalue "BP_Bullet_C") (!= _returnvalue "/Game/Kim/TopDown/Blueprints/BP_TopDownCharacter.BP_TopDownCharacter_C"))
    (Actor|DestroyActor)))

(event OnComponentBeginOverlap(Sphere)
  (params (OverlappedComponent :type Primitive%20Component%20Object%20Reference) (OtherActor :type Actor%20Object%20Reference) (OtherComp :type Primitive%20Component%20Object%20Reference) (OtherBodyIndex :type Integer) (bFromSweep :type Boolean) (SweepResult :type Hit%20Result%20Structure%20%28by%20ref%29))
  (if (not (Actor|ActorHasTag (.hitactor SweepResult) "Player"))
    (Effects|SpawnEmitteratLocation "/Game/Resources/StarterContent/Particles/P_Explosion.P_Explosion" (Transformation|GetWorldLocation (Variables|Default|GetSphere)))
    (Game|Damage|ApplyDamage (.hitactor SweepResult) 1.0 0 (Components|GetOwner))
    (Actor|DestroyActor)))

(event EventBeginPlay
  (Actor|SetLifeSpan (Variables|Default|GetLifeTime)))

(fn ConstructionScript)